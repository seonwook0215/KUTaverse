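; KUTaverse game mode that sets up the local player's VRoid avatar and mobile touch controls at startup.
; BeginPlay swaps the skeletal mesh by the game instance's character type, requests the user's inventory by email via VaRest, and enables a left virtual joystick.
; The response callback stores owned and equipped items in KUGameInstance, then maps equipped IDs to aura overlay materials and Niagara effects, or a rocket exhaust.
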(event `self.ReceiveBeginPlay`
  (bind _returnvalue (subsystem `VaRestSubsystem`))
  (`|ExecutionSequence`
    (:`then_0`
      (bind _askugame_instance (cast `KUGameInstance` (`GameplayStatics.GetGameInstance`)))
      (bind _returnvalue_2 (`KUGameInstance.GetUserCharacterType` _askugame_instance))
      (`KismetSystemLibrary.PrintString` _returnvalue_2)
      (if (`KismetStringLibrary.EqualEqual_StrStr` _returnvalue_2 "MALE")
        (bind _asbp_vroid_character (cast `/Game/VRoid_Character/BP_VRoidCharacter` (`GameplayStatics.GetPlayerCharacter` 0)))
        (`SkeletalMeshComponent.SetSkeletalMeshAsset` (`Character.Mesh` _asbp_vroid_character) "/Game/VRoid_Character/Male/First/SK_VRoid_Test2.SK_VRoid_Test2")
        (else
          (bind _asbp_vroid_character_2 (cast `/Game/VRoid_Character/BP_VRoidCharacter` (`GameplayStatics.GetPlayerCharacter` 0)))
          (`SkeletalMeshComponent.SetSkeletalMeshAsset` (`Character.Mesh` _asbp_vroid_character_2) "/Game/VRoid_Character/Female/First/SK_VRoid_Test1.SK_VRoid_Test1"))))
    (:`then_1`
      (bind _askugame_instance_2 (cast `KUGameInstance` (`GameplayStatics.GetGameInstance`)))
      (bind _returnvalue_3 (`VaRestSubsystem.ConstructVaRestJsonObject` _returnvalue))
      (`VaRestSubsystem.CallURL` _returnvalue (`KismetTextLibrary.Conv_TextToString` (`|FormatText` "https://kutaverse.xyz/user-service/inventorys?email={email}" (`KUGameInstance.GetUserEmail` _askugame_instance_2))) "GET" "json" _returnvalue_3 (delegate `InventoryEvent`)))
    (:`then_2`
      (`PlayerController.ActivateTouchInterface` (`GameplayStatics.GetPlayerController` 0) "/Engine/MobileResources/HUD/LeftVirtualJoystickOnly.LeftVirtualJoystickOnly"))))

(event `InventoryEvent`
  (params (Request :type "VaRestRequestJSON Object Reference"))
  (bind _returnvalue (`VaRestJsonValue.AsObject` (`VaRestJsonObject.GetField` (`VaRestRequestJSON.GetResponseObject` Request) "response")))
  (for _array_element (`VaRestJsonObject.GetArrayField` _returnvalue "itemList")
    (bind _askugame_instance (cast `KUGameInstance` (`GameplayStatics.GetGameInstance`)))
    (`KUGameInstance.SetInventoryArr` _askugame_instance (`KismetMathLibrary.FTrunc` (`VaRestJsonValue.AsNumber` _array_element))))
  (for (_array_element_2 _array_index) (`VaRestJsonObject.GetArrayField` _returnvalue "useItemList")
    (bind _askugame_instance_2 (cast `KUGameInstance` (`GameplayStatics.GetGameInstance`)))
    (`KUGameInstance.SetEquipArr` _askugame_instance_2 _array_index (`KismetMathLibrary.FTrunc` (`VaRestJsonValue.AsNumber` _array_element_2))))
  (bind _askugame_instance_3 (cast `KUGameInstance` (`GameplayStatics.GetGameInstance`)))
  (bind _returnvalue_2 (`KUGameInstance.GetEquipArr` _askugame_instance_3))
  (for _array_element_3 _returnvalue_2
    (switch `int` _array_element_3
      (:`1`
        (bind _asbp_vroid_character (cast `/Game/VRoid_Character/BP_VRoidCharacter` (`GameplayStatics.GetPlayerCharacter` 0)))
        (`MeshComponent.SetOverlayMaterial` (`Character.Mesh` _asbp_vroid_character) "/Game/Aura/M_Aura_Red.M_Aura_Red")
        (bind _asbp_vroid_character_2 (cast `/Game/VRoid_Character/BP_VRoidCharacter` (`GameplayStatics.GetPlayerCharacter` 0)))
        (`NiagaraComponent.SetAsset` (`/Game/VRoid_Character/BP_VRoidCharacter.Niagara_P` _asbp_vroid_character_2) null true)
        (`NiagaraComponent.SetAsset` (`/Game/VRoid_Character/BP_VRoidCharacter.Niagara` _asbp_vroid_character_2) "/Game/Aura/NS_Aura_Red.NS_Aura_Red" true))
      (:`2`
        (bind _asbp_vroid_character_3 (cast `/Game/VRoid_Character/BP_VRoidCharacter` (`GameplayStatics.GetPlayerCharacter` 0)))
        (`MeshComponent.SetOverlayMaterial` (`Character.Mesh` _asbp_vroid_character_3) "/Game/Aura/M_Aura_Blue.M_Aura_Blue")
        (bind _asbp_vroid_character_4 (cast `/Game/VRoid_Character/BP_VRoidCharacter` (`GameplayStatics.GetPlayerCharacter` 0)))
        (`NiagaraComponent.SetAsset` (`/Game/VRoid_Character/BP_VRoidCharacter.Niagara_P` _asbp_vroid_character_4) null true)
        (`NiagaraComponent.SetAsset` (`/Game/VRoid_Character/BP_VRoidCharacter.Niagara` _asbp_vroid_character_4) "/Game/Aura/NS_Aura_Blue.NS_Aura_Blue" true))
      (:`3`
        (bind _asbp_vroid_character_5 (cast `/Game/VRoid_Character/BP_VRoidCharacter` (`GameplayStatics.GetPlayerCharacter` 0)))
        (`MeshComponent.SetOverlayMaterial` (`Character.Mesh` _asbp_vroid_character_5) "/Game/Aura/M_Aura_Black.M_Aura_Black")
        (bind _asbp_vroid_character_6 (cast `/Game/VRoid_Character/BP_VRoidCharacter` (`GameplayStatics.GetPlayerCharacter` 0)))
        (`NiagaraComponent.SetAsset` (`/Game/VRoid_Character/BP_VRoidCharacter.Niagara_P` _asbp_vroid_character_6) null true)
        (`NiagaraComponent.SetAsset` (`/Game/VRoid_Character/BP_VRoidCharacter.Niagara` _asbp_vroid_character_6) "/Game/Aura/NS_Aura_Black.NS_Aura_Black" true))
      (:`4`
        (bind _asbp_vroid_character_7 (cast `/Game/VRoid_Character/BP_VRoidCharacter` (`GameplayStatics.GetPlayerCharacter` 0)))
        (`MeshComponent.SetOverlayMaterial` (`Character.Mesh` _asbp_vroid_character_7) null)
        (bind _asbp_vroid_character_8 (cast `/Game/VRoid_Character/BP_VRoidCharacter` (`GameplayStatics.GetPlayerCharacter` 0)))
        (`NiagaraComponent.SetAsset` (`/Game/VRoid_Character/BP_VRoidCharacter.Niagara_P` _asbp_vroid_character_8) "/Game/RocketThrusterExhaustFX/FX/NS_RocketExhaust_Violet.NS_RocketExhaust_Violet" true)
        (`NiagaraComponent.SetAsset` (`/Game/VRoid_Character/BP_VRoidCharacter.Niagara` _asbp_vroid_character_8) null true)))))

(fn `UserConstructionScript`)