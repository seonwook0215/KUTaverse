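; Player duck for a rhythm mini-game where the player copies a random direction sequence shown by an AI duck.
; BeginPlay chains four levels of increasing length and speed through nested delayed-loop macros, switching tagged cameras between AI demonstration and player turn.
; AddArr records choices, CalScore counts positional matches, and Tick computes the input-time fraction.
; Dialogue widgets open and close the game, with CreateDialogue grading the score, before loading Engineer_Building.
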(event `self.ReceiveBeginPlay`
  (bind _count (`self.Count`))
  (bind _count_2 (`self.Count`))
  (bind _count_3 (`self.Count`))
  (bind _count_4 (`self.Count`))
  (`PlayerController.ActivateTouchInterface` (`GameplayStatics.GetPlayerController` 0) null)
  (bind _outactors (`GameplayStatics.GetAllActorsWithTag` "Cam1"))
  (set `self.AICamera` (`|GetArrayItem` _outactors))
  (bind _outactors_2 (`GameplayStatics.GetAllActorsWithTag` "Cam2"))
  (set `self.PlayerCamera` (`|GetArrayItem` _outactors_2))
  (bind _outactors_3 (`GameplayStatics.GetAllActorsWithTag` "Cam3"))
  (set `self.AICamera2` (`|GetArrayItem` _outactors_3))
  (bind _outactors_4 (`GameplayStatics.GetAllActorsWithTag` "AIDuck"))
  (set `self.AIDuck` (`|GetArrayItem` _outactors_4))
  (set `self.Score` 0)
  (`self.ClearArr`)
  (`self.ShowAIClose`)
  (bind _returnvalue (`|CreateWidget` "/Game/Blueprints/MiniGame/Rhythm/WG_RhythmMiniGame2.WG_RhythmMiniGame2_C"))
  (bind _output_get (set `self.DuckDialogue` _returnvalue))
  (`UserWidget.AddToViewport` _output_get 0)
  (`KismetSystemLibrary.Delay` 4.0)
  (`Widget.RemoveFromParent` (`self.DuckDialogue`))
  (set `self.FirstDialogue` false)
  (bind _returnvalue_2 (`|CreateWidget` "/Game/Blueprints/MiniGame/Rhythm/WG_RhythmMiniGame.WG_RhythmMiniGame_C" (`GameplayStatics.GetPlayerController` 0)))
  (set `self.Rhythm_WG` _returnvalue_2)
  (`UserWidget.AddToViewport` _returnvalue_2 0)
  ;[1 1 1] Level0
  (`self.Level0`)
  (bind _index (`self.ForLoopWithDelay` 0 1 (`self.FullTimer`))
    (:`Last Body`
      (if (not (== _index 0))
        (`self.CalScore`)
        (`Widget.RemoveFromParent` (`self.ProgressbarWidget`)))
      (`self.ShowAI`)
      (`KismetSystemLibrary.Delay` 1.5)
      (bind _askuduck_character (cast `KUDuckCharacter` (`self.AIDuck`)))
      (`self.AIRand` _count_4)
      (bind _index_2 (`self.ForLoopWithDelay` 0 _count_4 (`self.AIShowTimer`))
        (:`Last Body`
          (`self.UpdateAnimationDirection` _askuduck_character "IDLE")
          (`self.UpdateAnimationDirection` _askuduck_character (`|GetArrayItem` (`self.NewDirectionArr`) _index_2))
          (`self.UpdateAnimationDirection` (stale _askuduck_character_2) "IDLE"))
        (:`Completed`
          (`KismetSystemLibrary.Delay` 0.5)
          (`self.ClearArr`)
          (`self.UpdateAnimationDirection` _askuduck_character "IDLE")
          (bind _askuduck_character_2 (cast `KUDuckCharacter` (`GameplayStatics.GetPlayerCharacter` 0)))
          (`self.MakeTimeZero` _askuduck_character_2)
          (bind _returnvalue_3 (`|CreateWidget` "/Game/Blueprints/MiniGame/Rhythm/WG_RhythmMiniGame1.WG_RhythmMiniGame1_C" (`GameplayStatics.GetPlayerController` 0)))
          (bind _output_get_2 (set `self.ProgressbarWidget` _returnvalue_3))
          (`UserWidget.AddToViewport` _output_get_2 0)
          (`self.ShowPlayer`))))
    (:`Completed`
      (`self.CalScore`)
      (`Widget.RemoveFromParent` (`self.ProgressbarWidget`))
      ;[1 1 1] Level1
      (`self.Level1`)
      (bind _index_3 (`self.ForLoopWithDelay` 0 2 (`self.FullTimer`))
        (:`Last Body`
          (if (not (== _index_3 0))
            (`self.CalScore`)
            (`Widget.RemoveFromParent` (`self.ProgressbarWidget`)))
          (`self.ShowAI`)
          (`KismetSystemLibrary.Delay` 1.5)
          (bind _askuduck_character_3 (cast `KUDuckCharacter` (`self.AIDuck`)))
          (`self.AIRand` _count)
          (bind _index_4 (`self.ForLoopWithDelay` 0 _count (`self.AIShowTimer`))
            (:`Last Body`
              (`self.UpdateAnimationDirection` _askuduck_character_3 "IDLE")
              (`self.UpdateAnimationDirection` _askuduck_character_3 (`|GetArrayItem` (`self.NewDirectionArr`) _index_4))
              (`self.UpdateAnimationDirection` (stale _askuduck_character_4) "IDLE"))
            (:`Completed`
              (`KismetSystemLibrary.Delay` 0.5)
              (`self.ClearArr`)
              (`self.UpdateAnimationDirection` _askuduck_character_3 "IDLE")
              (bind _askuduck_character_4 (cast `KUDuckCharacter` (`GameplayStatics.GetPlayerCharacter` 0)))
              (`self.MakeTimeZero` _askuduck_character_4)
              (bind _returnvalue_4 (`|CreateWidget` "/Game/Blueprints/MiniGame/Rhythm/WG_RhythmMiniGame1.WG_RhythmMiniGame1_C" (`GameplayStatics.GetPlayerController` 0)))
              (bind _output_get_3 (set `self.ProgressbarWidget` _returnvalue_4))
              (`UserWidget.AddToViewport` _output_get_3 0)
              (`self.ShowPlayer`))))
        (:`Completed`
          (`self.CalScore`)
          (`Widget.RemoveFromParent` (`self.ProgressbarWidget`))
          ;[1 1 1] Level2
          (`self.Level2`)
          (bind _index_5 (`self.ForLoopWithDelay` 0 2 (`self.FullTimer`))
            (:`Last Body`
              (if (not (== _index_5 0))
                (`self.CalScore`)
                (`Widget.RemoveFromParent` (`self.ProgressbarWidget`)))
              (`self.ShowAI`)
              (`KismetSystemLibrary.Delay` 1.5)
              (bind _askuduck_character_5 (cast `KUDuckCharacter` (`self.AIDuck`)))
              (`self.AIRand` _count_3)
              (bind _index_6 (`self.ForLoopWithDelay` 0 _count_3 (`self.AIShowTimer`))
                (:`Last Body`
                  (`self.UpdateAnimationDirection` _askuduck_character_5 "IDLE")
                  (`self.UpdateAnimationDirection` _askuduck_character_5 (`|GetArrayItem` (`self.NewDirectionArr`) _index_6))
                  (`self.UpdateAnimationDirection` (stale _askuduck_character_6) "IDLE"))
                (:`Completed`
                  (`KismetSystemLibrary.Delay` 0.5)
                  (`self.ClearArr`)
                  (`self.UpdateAnimationDirection` _askuduck_character_5 "IDLE")
                  (bind _askuduck_character_6 (cast `KUDuckCharacter` (`GameplayStatics.GetPlayerCharacter` 0)))
                  (`self.MakeTimeZero` _askuduck_character_6)
                  (bind _returnvalue_5 (`|CreateWidget` "/Game/Blueprints/MiniGame/Rhythm/WG_RhythmMiniGame1.WG_RhythmMiniGame1_C" (`GameplayStatics.GetPlayerController` 0)))
                  (bind _output_get_4 (set `self.ProgressbarWidget` _returnvalue_5))
                  (`UserWidget.AddToViewport` _output_get_4 0)
                  (`self.ShowPlayer`))))
            (:`Completed`
              (`self.CalScore`)
              (`Widget.RemoveFromParent` (`self.ProgressbarWidget`))
              ;[1 1 1] Level3
              (`self.Level3`)
              (bind _index_7 (`self.ForLoopWithDelay` 0 3 (`self.FullTimer`))
                (:`Last Body`
                  (if (not (== _index_7 0))
                    (`self.CalScore`)
                    (`Widget.RemoveFromParent` (`self.ProgressbarWidget`)))
                  (`self.ShowAI`)
                  (`KismetSystemLibrary.Delay` 1.5)
                  (bind _askuduck_character_7 (cast `KUDuckCharacter` (`self.AIDuck`)))
                  (`self.AIRand` _count_2)
                  (bind _index_8 (`self.ForLoopWithDelay` 0 _count_2 (`self.AIShowTimer`))
                    (:`Last Body`
                      (`self.UpdateAnimationDirection` _askuduck_character_7 "IDLE")
                      (`self.UpdateAnimationDirection` _askuduck_character_7 (`|GetArrayItem` (`self.NewDirectionArr`) _index_8))
                      (`self.UpdateAnimationDirection` (stale _askuduck_character_8) "IDLE"))
                    (:`Completed`
                      (`KismetSystemLibrary.Delay` 0.5)
                      (`self.ClearArr`)
                      (`self.UpdateAnimationDirection` _askuduck_character_7 "IDLE")
                      (bind _askuduck_character_8 (cast `KUDuckCharacter` (`GameplayStatics.GetPlayerCharacter` 0)))
                      (`self.MakeTimeZero` _askuduck_character_8)
                      (bind _returnvalue_6 (`|CreateWidget` "/Game/Blueprints/MiniGame/Rhythm/WG_RhythmMiniGame1.WG_RhythmMiniGame1_C" (`GameplayStatics.GetPlayerController` 0)))
                      (bind _output_get_5 (set `self.ProgressbarWidget` _returnvalue_6))
                      (`UserWidget.AddToViewport` _output_get_5 0)
                      (`self.ShowPlayer`))))
                (:`Completed`
                  (`Widget.RemoveFromParent` (`self.Rhythm_WG`))
                  (`self.ShowAIClose`)
                  (bind _returnvalue_7 (`|CreateWidget` "/Game/Blueprints/MiniGame/Rhythm/WG_RhythmMiniGame2.WG_RhythmMiniGame2_C"))
                  (bind _output_get_6 (set `self.DuckDialogue` _returnvalue_7))
                  (`UserWidget.AddToViewport` _output_get_6 0)
                  (`KismetSystemLibrary.Delay` 5.0)
                  (`GameplayStatics.OpenLevel` "Engineer_Building"))))))))))

(event `self.ReceiveTick`
  (params (DeltaSeconds :type "Float (single-precision)"))
  ;[1 1 1] Timer
  (bind _askuduck_character (cast `KUDuckCharacter` (`GameplayStatics.GetPlayerCharacter` 0)))
  (bind _returnvalue (`self.ReturnTimeZero` _askuduck_character))
  (set `self.PlayerPlayTimer` (/ (- (- (`self.FullTimer`) (+ (* (`self.AIShowTimer`) (`self.Count`)) 3.5)) _returnvalue) (- (`self.FullTimer`) (+ (* (`self.AIShowTimer`) (`self.Count`)) 3.5)))))

(fn `AddArr`
  (params (PlayerChoose :type "EDirection Enum" :default "IDLE"))
  (returns (Check :type Boolean))
  (if (>= (`self.Count`) (`KismetArrayLibrary.Array_Length` (`self.PlayerDirectionArr`)))
    (`KismetArrayLibrary.Array_Add` (`self.PlayerDirectionArr`) PlayerChoose)
    (return true)
    (else
      (`KismetSystemLibrary.PrintString` "YouCant")
      (return false))))

(fn `AIRand`
  (params (Count :type Integer))
  (`KismetArrayLibrary.Array_Clear` (`self.NewDirectionArr`))
  (for _ (range (+ Count 1))
    (switch `int` (`KismetMathLibrary.RandomInteger` 3)
      (:`0`
        (set `self.NewDirection` "UP"))
      (:`1`
        (set `self.NewDirection` "DOWN"))
      (:`2`
        (set `self.NewDirection` "LEFT"))
      (:`3`
        (bind _output_get (set `self.NewDirection` "RIGHT"))))
    (`KismetArrayLibrary.Array_Add` (`self.NewDirectionArr`) _output_get)))

(fn `CalScore`
  (for _index (range (+ (`self.Count`) 1))
    (if (`|EnumEquality` (`|GetArrayItem` (`self.NewDirectionArr`) _index) (`|GetArrayItem` (`self.PlayerDirectionArr`) _index))
      (bind _result (`/Engine/EditorBlueprintResources/StandardMacros.IncrementInt` (`self.Score`))
        (:`  `
          (set `self.Score` _result))))))

(fn `ClearArr`
  (`KismetArrayLibrary.Array_Clear` (`self.PlayerDirectionArr`)))

(fn `CreateDialogue`
  (returns (NewParam :type String))
  (locals (Dialogue :type String :default "날 따라하도록"))
  (if (`self.FirstDialogue`)
    (return (`local.Dialogue`))
    (elif (<= (`self.Score`) 7)
      (bind _output_get (set `local.Dialogue` "자네 실력이 형편 없군!"))
      (return _output_get)
      (elif (<= (`self.Score`) 12)
        (bind _output_get_2 (set `local.Dialogue` "좀 더 분발할 수 있도록..."))
        (return _output_get_2)
        (elif (<= (`self.Score`) 18)
          (bind _output_get_3 (set `local.Dialogue` "이 정도면 나쁘지 않군."))
          (return _output_get_3)
          (elif (<= (`self.Score`) 25)
            (bind _output_get_4 (set `local.Dialogue` "아주 좋아!! 그대로만 하게"))
            (return _output_get_4)
            (else
              (bind _output_get_5 (set `local.Dialogue` "나를 뛰어 넘었군. 합격이다!"))
              (return _output_get_5))))))))

(fn `Level0`
  (set `self.Count` 1)
  (set `self.FullTimer` 8.0)
  (set `self.AIShowTimer` 1.0))

(fn `Level1`
  (set `self.Count` 2)
  (set `self.FullTimer` 8.0)
  (set `self.AIShowTimer` 1.0))

(fn `Level2`
  (set `self.Count` 3)
  (set `self.FullTimer` 8.0)
  (set `self.AIShowTimer` 0.75))

(fn `Level3`
  (set `self.Count` 4)
  (set `self.FullTimer` 7.0)
  (set `self.AIShowTimer` 0.5))

(fn `ShowAI`
  (`PlayerController.SetViewTargetWithBlend` (`GameplayStatics.GetPlayerController` 0) (`self.AICamera`) 0.5 "VTBlend_Linear" 0.0 false))

(fn `ShowAIClose`
  (`PlayerController.SetViewTargetWithBlend` (`GameplayStatics.GetPlayerController` 0) (`self.AICamera2`) 0.25 "VTBlend_Linear" 0.0 false))

(fn `ShowPlayer`
  (`PlayerController.SetViewTargetWithBlend` (`GameplayStatics.GetPlayerController` 0) (`self.PlayerCamera`) 0.5 "VTBlend_Linear" 0.0 false))

(fn `UserConstructionScript`)