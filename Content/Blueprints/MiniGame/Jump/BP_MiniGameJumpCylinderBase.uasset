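; BP_MiniGameJumpCylinderBase is a cylinder platform for the jump minigame that awards points and then drops away.
; The player's first overlap with its Box, gated by FirstTouched, adds a fixed score to BP_MiniGamePersonReal.
; After a short delay, a Timeline lowers the actor by subtracting its track value from Z on each update.
; ForwardMove shifts the actor along negative X by a passed amount.
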(event `self.ReceiveBeginPlay`)

(event `self.Box.OnComponentBeginOverlap`
  (params (OverlappedComponent :type "PrimitiveComponent Object Reference") (OtherActor :type "Actor Object Reference") (OtherComp :type "PrimitiveComponent Object Reference") (OtherBodyIndex :type Integer) (bFromSweep :type Boolean) (SweepResult :type "HitResult Structure (by ref)"))
  (if (== OtherActor (`GameplayStatics.GetPlayerCharacter` 0))
    (if (`self.FirstTouched`)
      (set `self.FirstTouched` false)
      (bind _asbp_mini_game_person_real (cast `/Game/Blueprints/MiniGame/Jump/BP_MiniGamePersonReal` (`GameplayStatics.GetPlayerCharacter` 0)))
      (set `/Game/Blueprints/MiniGame/Jump/BP_MiniGamePersonReal.Score` (+ (`/Game/Blueprints/MiniGame/Jump/BP_MiniGamePersonReal.Score` _asbp_mini_game_person_real) 10) _asbp_mini_game_person_real)
      (`KismetSystemLibrary.Delay` 3.0)
      (bind (_direction _newtrack_4) (`Timeline|Timeline` :!via `PlayFromStart`)
        (:`Update`
          (`self.K2_SetActorLocation` (`KismetMathLibrary.MakeVector` (.x (`self.K2_GetActorLocation`)) (.y (`self.K2_GetActorLocation`)) (- (.z (`self.K2_GetActorLocation`)) _newtrack_4))))))))

(fn `ForwardMove`
  (params (NewParam :type "Float (double-precision)"))
  (`self.K2_SetActorLocation` (`KismetMathLibrary.MakeVector` (- (.x (`self.K2_GetActorLocation`)) NewParam) (.y (`self.K2_GetActorLocation`)) (.z (`self.K2_GetActorLocation`)))))

(fn `UserConstructionScript`)