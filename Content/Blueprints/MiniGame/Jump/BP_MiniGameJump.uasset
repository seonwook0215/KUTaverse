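; BP_MiniGameJump runs the jump minigame, generating an endless platform course along X as the player advances.
; BeginPlay finds the tagged camera, enables touch input and picks the player mesh from the saved gender.
; Tick spawns chunks of ten randomly offset static or moving cylinders, occasional coins over static ones, and a rest platform.
; It also destroys root components of coins and cylinders behind the camera, leaving rest platforms untouched.
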(event `self.ReceiveBeginPlay`
  (`PlayerController.ActivateTouchInterface` (`GameplayStatics.GetPlayerController` 0) null)
  (bind _outactors (`GameplayStatics.GetAllActorsWithTag` "Cam1"))
  (set `self.PlayerCamera` (`|GetArrayItem` _outactors))
  (set `PlayerController.bShowMouseCursor` false (`GameplayStatics.GetPlayerController` 0))
  (bind _asbp_mini_game_person_real (cast `/Game/Blueprints/MiniGame/Jump/BP_MiniGamePersonReal` (`GameplayStatics.GetPlayerCharacter` 0)))
  (bind _askugame_instance (cast `KUGameInstance` (`GameplayStatics.GetGameInstance`)))
  (if (`KismetStringLibrary.EqualEqual_StrStr` (`KUGameInstance.GetUserCharacterType` _askugame_instance) "MALE")
    (bind _mesh (`Character.Mesh` _asbp_mini_game_person_real))
    (`SkeletalMeshComponent.SetSkeletalMeshAsset` _mesh "/Game/VRoid_Character/Male/First/SK_VRoid_Test2.SK_VRoid_Test2")
    (else
      (`SkeletalMeshComponent.SetSkeletalMeshAsset` _mesh "/Game/VRoid_Character/Female/First/SK_VRoid_Test1.SK_VRoid_Test1"))))

(event `self.ReceiveTick`
  (params (DeltaSeconds :type "Float (single-precision)"))
  (`|ExecutionSequence`
    (:`then_0`
      (if (< (`self.MakeBlock`) (+ (.x (`self.K2_GetActorLocation` (`GameplayStatics.GetPlayerCharacter` 0))) (`self.Far`)))
        (set `self.MakeBlock` (+ (`self.MakeBlock`) (`self.Far`)))
        (for _index (range 10)
          (if (> 2 (`KismetMathLibrary.RandomInteger` 10))
            (`|SpawnActorFromClass` "/Game/Blueprints/MiniGame/Jump/BP_MiniGameJumpCylinderMove.BP_MiniGameJumpCylinderMove_C" (`KismetMathLibrary.Conv_VectorToTransform` (`KismetMathLibrary.MakeVector` (+ (`self.MakeBlock`) (* _index 250)) (`KismetMathLibrary.RandomFloatInRange` -350.0 350.0) -158.0)) "AlwaysSpawn" "MultiplyWithRoot" null null)
            (else
              (bind _returnvalue (`|SpawnActorFromClass` "/Game/Blueprints/MiniGame/Jump/BP_MiniGameJumpCylinderBase.BP_MiniGameJumpCylinderBase_C" (`KismetMathLibrary.Conv_VectorToTransform` (`KismetMathLibrary.MakeVector` (+ (`self.MakeBlock`) (* _index 250)) (`KismetMathLibrary.RandomFloatInRange` -350.0 350.0) -158.0)) "AlwaysSpawn" "MultiplyWithRoot" null null))
              (if (> (`self.MakeCoin`) (`KismetMathLibrary.RandomInteger` 100))
                (`|SpawnActorFromClass` "/Game/Blueprints/MiniGame/Jump/BP_MiniGameJumpCoin.BP_MiniGameJumpCoin_C" (`KismetMathLibrary.Conv_VectorToTransform` (`KismetMathLibrary.MakeVector` (.x (`self.K2_GetActorLocation` _returnvalue)) (.y (`self.K2_GetActorLocation` _returnvalue)) 200.0)) "AlwaysSpawn" "MultiplyWithRoot" null null)))))
        (`|SpawnActorFromClass` "/Game/Blueprints/MiniGame/Jump/BP_MiniGameJumpRest.BP_MiniGameJumpRest_C" (`KismetMathLibrary.Conv_VectorToTransform` (`KismetMathLibrary.MakeVector` (+ (`self.MakeBlock`) (* 10.0 250)) 0.0 -158.0)) "Undefined" "MultiplyWithRoot" null null)))
    (:`then_1`
      (`|ExecutionSequence`
        (:`then_0`
          (bind _outactors (`GameplayStatics.GetAllActorsOfClass` "/Game/Blueprints/MiniGame/Jump/BP_MiniGameJumpCoin.BP_MiniGameJumpCoin_C"))
          (for _array_element _outactors
            (if (> (- (.x (`self.K2_GetActorLocation` (`self.PlayerCamera`))) 500.0) (.x (`self.K2_GetActorLocation` _array_element)))
              (`ActorComponent.K2_DestroyComponent` (`Actor.RootComponent` _array_element)))))
        (:`then_1`
          (bind _outactors_2 (`GameplayStatics.GetAllActorsOfClass` "/Game/Blueprints/MiniGame/Jump/BP_MiniGameJumpCylinderBase.BP_MiniGameJumpCylinderBase_C"))
          (for _array_element_2 _outactors_2
            (if (> (- (.x (`self.K2_GetActorLocation` (`self.PlayerCamera`))) 500.0) (.x (`self.K2_GetActorLocation` _array_element_2)))
              (`ActorComponent.K2_DestroyComponent` (`Actor.RootComponent` _array_element_2)))))
        (:`then_2`
          (bind _outactors_3 (`GameplayStatics.GetAllActorsOfClass` "/Game/Blueprints/MiniGame/Jump/BP_MiniGameJumpCylinderMove.BP_MiniGameJumpCylinderMove_C"))
          (for _array_element_3 _outactors_3
            (if (> (- (.x (`self.K2_GetActorLocation` (`self.PlayerCamera`))) 500.0) (.x (`self.K2_GetActorLocation` _array_element_3)))
              (`ActorComponent.K2_DestroyComponent` (`Actor.RootComponent` _array_element_3)))))))))

(fn `UserConstructionScript`)