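; BP_MiniGameJumpRest is a rest object in the jump minigame that rewards the player on first contact.
; Its box overlap casts the player to BP_MiniGamePersonReal, adds score and advances a rest counter, raising Level on every third rest.
; A FirstTouched flag limits the reward to once per instance.
; ForwardMove shifts the actor along negative world X by a given distance, without sweeping.
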(event `self.Box.OnComponentBeginOverlap`
  (params (OverlappedComponent :type "PrimitiveComponent Object Reference") (OtherActor :type "Actor Object Reference") (OtherComp :type "PrimitiveComponent Object Reference") (OtherBodyIndex :type Integer) (bFromSweep :type Boolean) (SweepResult :type "HitResult Structure (by ref)"))
  (if (== OtherActor (`GameplayStatics.GetPlayerCharacter` 0))
    (if (`self.FirstTouched`)
      (set `self.FirstTouched` false)
      (bind _asbp_mini_game_person_real (cast `/Game/Blueprints/MiniGame/Jump/BP_MiniGamePersonReal` (`GameplayStatics.GetPlayerCharacter` 0)))
      (set `/Game/Blueprints/MiniGame/Jump/BP_MiniGamePersonReal.Score` (+ (`/Game/Blueprints/MiniGame/Jump/BP_MiniGamePersonReal.Score` _asbp_mini_game_person_real) 100) _asbp_mini_game_person_real)
      (bind _returnvalue (+ (`/Game/Blueprints/MiniGame/Jump/BP_MiniGamePersonReal.RestCount` _asbp_mini_game_person_real) 1))
      (if (== _returnvalue 3)
        (set `/Game/Blueprints/MiniGame/Jump/BP_MiniGamePersonReal.RestCount` 0 _asbp_mini_game_person_real)
        (set `/Game/Blueprints/MiniGame/Jump/BP_MiniGamePersonReal.Level` (+ (`/Game/Blueprints/MiniGame/Jump/BP_MiniGamePersonReal.Level` _asbp_mini_game_person_real) 1) _asbp_mini_game_person_real)
        (else
          (set `/Game/Blueprints/MiniGame/Jump/BP_MiniGamePersonReal.RestCount` _returnvalue _asbp_mini_game_person_real))))))

(fn `ForwardMove`
  (params (NewParam :type "Float (double-precision)"))
  (`self.K2_SetActorLocation` (`KismetMathLibrary.MakeVector` (- (.x (`self.K2_GetActorLocation`)) NewParam) (.y (`self.K2_GetActorLocation`)) (.z (`self.K2_GetActorLocation`)))))

(fn `UserConstructionScript`)