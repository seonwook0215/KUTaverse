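; Player character for the jump minigame, with touch drag-and-release jumping and a coin counter.
; Dragging offsets a landing point from the character, and CalculateJump builds a three-point spline arc to it with a height-adjusted apex and a landing decal.
; Release plays a timeline that steers movement velocity along the spline, resetting after finish or landing.
; Tick keeps the tagged camera and water actors trailing the character along X.
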(event `InputAxis|MoveForward` :overrideparent false
  (params (AxisValue :type "Float (single-precision)"))
  (`self.AddMovementInput` (`KismetMathLibrary.GetForwardVector` (`KismetMathLibrary.MakeRotator` 0.0 0.0 (.yaw (`self.GetControlRotation`)))) AxisValue)
  (if (`self.ReadyToJump`) :!label _label
    (bind _canjump (`self.CalculateJump` false))
    (set `self.ReadyToJump` _canjump)))

(event `InputAxis|MoveRight` :overrideparent false
  (params (AxisValue :type "Float (single-precision)"))
  (`self.AddMovementInput` (`KismetMathLibrary.GetRightVector` (`KismetMathLibrary.MakeRotator` 0.0 0.0 (.yaw (`self.GetControlRotation`)))) AxisValue)
  (goto _label))

(event `self.ReceiveBeginPlay`
  (`PlayerController.ActivateTouchInterface` (`GameplayStatics.GetPlayerController` 0) null)
  (bind _outactors (`GameplayStatics.GetAllActorsWithTag` "Water1"))
  (set `self.Water` (`|GetArrayItem` _outactors))
  (bind _outactors_2 (`GameplayStatics.GetAllActorsWithTag` "Cam1"))
  (bind _output_get (set `self.PlayerCamera` (`|GetArrayItem` _outactors_2)))
  (`PlayerController.SetViewTargetWithBlend` (`GameplayStatics.GetPlayerController` 0) _output_get 0.0 "VTBlend_Linear" 0.0 false)
  (bind _returnvalue (`|CreateWidget` "/Game/Blueprints/MiniGame/Jump/UMG_MiniGameJump.UMG_MiniGameJump_C"))
  (`UserWidget.AddToViewport` _returnvalue 0)
  (set `PlayerController.bShowMouseCursor` false (`GameplayStatics.GetPlayerController` 0))
  (`self.ResetJump`)
  (`KismetSystemLibrary.ExecuteConsoleCommand` "show splines" null)
  (set `SplineComponent.Duration` 1.0 (`self.Spline`))
  (`TimelineComponent.SetPlayRate` (`self.TL_Jump`) (`self.JumpSpeed`)))

(event `InputTouch`
  (params (Location :type "Vector Structure") (FingerIndex :type "ETouchIndex Enum"))
  (bind _returnvalue (`self.K2_GetActorLocation`))
  (bind _returnvalue_2 (`self.K2_GetActorLocation`))
  (bind (_locationx _locationy) (`PlayerController.GetInputTouchState` (`GameplayStatics.GetPlayerController` 0) "Touch1"))
  (bind (_locationx_2 _locationy_2) (`PlayerController.GetInputTouchState` (`GameplayStatics.GetPlayerController` 0) "Touch1"))
  (bind _returnvalue_3 (not (`self.BIsFalling`)))
  (bind (_returnvalue_x _returnvalue_y) (`KismetMathLibrary.BreakVector2D` (- (`KismetMathLibrary.MakeVector2D` _locationx _locationy) (`self.TouchLocationStart`))))
  (:`Pressed`
    (if _returnvalue_3
      (set `self.TouchLocationStart` (`KismetMathLibrary.MakeVector2D` _locationx_2 _locationy_2))
      (set `self.JumpFrom` (`self.K2_GetActorLocation`))))
  (:`Released`
    (if _returnvalue_3
      (`|ExecutionSequence`
        (:`then_0`
          (set `self.ReadyToJump` false)
          (set `self.isJumping` true)
          (`self.Jump`))
        (:`then_1`
          (`GameplayStatics.PlaySound2D` "/Game/Blueprints/MiniGame/Jump/Sound/cartoon-jump-6462.cartoon-jump-6462" 1.0 1.0 0.0 null null)
          (bind (_direction _jumpalpha01) (`Timeline|TL_Jump` :!via `PlayFromStart`)
            (:`Update`
              (bind _returnvalue_4 (`SplineComponent.GetLocationAtTime` (`self.Spline`) _jumpalpha01 "World" false))
              (bind _output_get (set `MovementComponent.Velocity` (* (`KismetMathLibrary.GetDirectionUnitVector` _returnvalue _returnvalue_4) (* (`KismetMathLibrary.Vector_Distance` _returnvalue _returnvalue_4) 50.0)) (`self.CharacterMovement`)))
              (`self.AddMovementInput` _output_get))
            (:`Finished`
              (`KismetSystemLibrary.Delay` 0.2 :!label _label_2)
              (`self.ResetJump`)))))))
  (:`Moved`
    (if _returnvalue_3
      (set `self.JumpTo` (`KismetMathLibrary.MakeVector` (.x (+ (`KismetMathLibrary.MakeVector` (* _returnvalue_y 1.0) (* _returnvalue_x -1.0)) _returnvalue_2)) (.y (+ (`KismetMathLibrary.MakeVector` (* _returnvalue_y 1.0) (* _returnvalue_x -1.0)) _returnvalue_2)) (.z _returnvalue_2)))
      (`self.CalculateJump` false))))

(event `self.OnLanded`
  (params (Hit :type "HitResult Structure (by ref)"))
  (goto _label_2))

(event `self.ReceiveTick`
  (params (DeltaSeconds :type "Float (single-precision)"))
  (set `self.BIsFalling` (`NavMovementComponent.IsFalling` (`self.CharacterMovement`)))
  (`self.K2_SetActorLocation` (`self.PlayerCamera`) (`KismetMathLibrary.MakeVector` (- (.x (`self.K2_GetActorLocation`)) 1200.0) (.y (`self.K2_GetActorLocation` (`self.PlayerCamera`))) (.z (`self.K2_GetActorLocation` (`self.PlayerCamera`)))) false false)
  (`self.K2_SetActorLocation` (`self.Water`) (`KismetMathLibrary.MakeVector` (- (.x (`self.K2_GetActorLocation`)) 1200.0) (.y (`self.K2_GetActorLocation` (`self.Water`))) (.z (`self.K2_GetActorLocation` (`self.Water`)))) false false))

(fn `CalculateJump`
  (params (ChooseNewTarget :type Boolean) (ApexOffsetFromMouseWheel :type "Float (double-precision)"))
  (returns (CanJump :type Boolean))
  (bind (_minmaxjumpdistance_x _minmaxjumpdistance_y) (`KismetMathLibrary.BreakVector2D` (`self.MinMaxJumpDistance`)))
  (bind _jumpto (`self.JumpTo`))
  (bind _jumpdistance (`self.JumpDistance`))
  (bind (_bblockinghit _binitialoverlap _time _distance _location _impactpoint _normal) (`GameplayStatics.BreakHitResult` (`PlayerController.GetHitResultUnderCursorByChannel` (`GameplayStatics.GetPlayerController` 0) "TraceTypeQuery1" true)))
  (if ChooseNewTarget
    (bind _output_get (set `self.JumpTo` _location))
    (set `self.JumpLandNormal` _normal))
  (bind _output_get_2 (set `self.JumpDistance` (`KismetMathLibrary.Vector_Distance` _output_get (`self.K2_GetActorLocation`)))) ; jump distance with a min / max clamp (below)
  (set `self.ReadyToJump` (`KismetMathLibrary.InRange_FloatFloat` _output_get_2 _minmaxjumpdistance_x _minmaxjumpdistance_y)) ; can't jump if we exceed the clamp
  (bind _output_get_3 (set `self.JumpFrom` (`self.K2_GetActorLocation`)))
  (`SplineComponent.SetSplinePoints` (`self.Spline`) (`|MakeArray` _output_get_3 (+ (* (+ _output_get_3 _jumpto) 0.5) (`KismetMathLibrary.MakeVector` 0.0 0.0 (* (`self.SetApexOffset` (`local.ApexOffsetFromMouseWheel`)) _jumpdistance))) _jumpto) "World" true) ; spline points:\n\n0: player's current location\n1: derived from\n    - distance between 0 & 2\n    - fixed apex offset enfored by a clamp\n    - additional offset controlled by mouse wheel\n    - dynamic value dictated by elevation  delta\n2: hit from mouse world click
  (if (`self.isLandingVertical`)
    (`SplineComponent.SetTangentAtSplinePoint` (`self.Spline`) 2 (* (0.0 0.0 -1.0) (`KismetMathLibrary.FClamp` _jumpdistance 0.0 2000.0)) "World" true) ; optional, controlled by isLandingVertical\n\nT: 2nd point's tangent affected by distance of the jump \nF: basic arc with automatic tangents
  )
  (`SceneComponent.K2_SetWorldLocationAndRotation` (`self.Decal`) (`self.JumpTo`) (`KismetMathLibrary.Conv_VectorToRotator` (`self.JumpLandNormal`)) false false) ; place the decal on the jump destination
  (`self.ShowJumpLine`) ; currently the spline is visualised by debug, perhaps\na couple of spline mesh components can go here
  (return true))

(fn `GainCoin`
  (set `self.Coin` (+ (`self.Coin`) 1)))

(fn `ResetJump`
  (`|ExecutionSequence`
    (:`then_0`
      (bind _output_get (set `self.JumpTo` (0.0 0.0 0.0)))
      (set `self.JumpFrom` _output_get)
      (set `self.JumpDistance` 0.0)
      (bind _output_get_2 (set `self.ReadyToJump` false))
      (set `self.isJumping` _output_get_2))
    (:`then_1`
      (`SceneComponent.SetVisibility` (`self.Spline`) false true)
      (`SceneComponent.SetVisibility` (`self.Decal`) false true))))

(fn `SetApexOffset`
  (params (Axis :type "Float (double-precision)"))
  (returns (FinalApex :type "Float (double-precision)"))
  (bind (_returnvalue_x _returnvalue_y _returnvalue_z) (`KismetMathLibrary.BreakVector` (`self.K2_GetActorLocation`)))
  (bind (_minmaxapexclamp_x _minmaxapexclamp_y) (`KismetMathLibrary.BreakVector2D` (`self.MinMaxApexClamp`)))
  (bind (_jumpto_x _jumpto_y _jumpto_z) (`KismetMathLibrary.BreakVector` (`self.JumpTo`)))
  (bind _output_get (set `self.ManualApexOffset` (`KismetMathLibrary.FClamp` (+ (* Axis 0.05) (`self.ManualApexOffset`)) _minmaxapexclamp_x _minmaxapexclamp_y))) ; accumulated fixed offset from mouse wheel
  (return (+ _output_get (`KismetMathLibrary.MapRangeClamped` (- _jumpto_z _returnvalue_z) 0.0 1000.0 0.0 1.0))))

(fn `ShowJumpLine`
  (`SceneComponent.SetVisibility` (`self.Decal`) true true)
  (`SceneComponent.SetVisibility` (`self.Spline`) true true))

(fn `UserConstructionScript`)