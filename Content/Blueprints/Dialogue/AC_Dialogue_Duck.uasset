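; Dialogue component for the tone-deaf duck NPC (음치 건덕), who asks the player for help singing at a festival.
; The Dialogue override calls its parent, then branches on DialogueTreeIndex into first meeting, return after refusal, or random greeting after acceptance.
; Accepting advances the index and opens the MiniGame_Rhythm level, with only the first-meeting path calling ActivateTouchInterface beforehand.
; Other endings clear or rewind dialogue progress before closing the conversation.
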(fn `Dialogue`
  (`parent.Dialogue`)
  (switch `int` (`self.DialogueTreeIndex`)
    (:`0`
      ;[1 1 1] Comment
      (bind (_state _optionindex) (`self.AddDialogue` "음치 건덕" "꽉 꽉 꽉(건덕이가 할말이 있어 보인다.)" (`|MakeArray` "들어본다." "듣지 않는다." :!type "Text")))
      (switch `/Game/Blueprints/Dialogue/Enum_DialogueState` _state
        (:`NewEnumerator0`
          (switch `int` _optionindex
            (:`0`
              ;[1 1 1] Comment
              (bind (_state_2 _optionindex_2) (`self.AddDialogue` "음치 건덕" "꽉 꽉 꽉꽉 꽉 꽉(들어봐. 축제 대표로 노래를 부르고 싶은데 그게 잘 되지가 않아... 너가 좀 도와줄래?)" (`|MakeArray` "그래!" "아니..." :!type "Text")))
              (switch `/Game/Blueprints/Dialogue/Enum_DialogueState` _state_2
                (:`NewEnumerator0`
                  (switch `int` _optionindex_2
                    (:`0`
                      ;[1 1 1] Comment
                      (bind _state_3 (`self.AddDialogue` "음치 건덕" "꽉꽉!(좋았어 가보는거야!)" (`|MakeArray` "(미니게임 플레이)" :!type "Text")))
                      (switch `/Game/Blueprints/Dialogue/Enum_DialogueState` _state_3
                        (:`NewEnumerator0`
                          (`self.SetDialogueTreeIndex` 2)
                          (`self.CloseConversation`)
                          (`PlayerController.ActivateTouchInterface` (`GameplayStatics.GetPlayerController` 0) null)
                          (`GameplayStatics.OpenLevel` "MiniGame_Rhythm"))))
                    (:`1`
                      ;[1 1 1] Comment
                      (bind _state_4 (`self.AddDialogue` "음치 건덕" "꽈악...(에휴...)" (`|MakeArray` "대화 끝내기" :!type "Text")))
                      (switch `/Game/Blueprints/Dialogue/Enum_DialogueState` _state_4
                        (:`NewEnumerator0`
                          (`self.SetDialogueTreeIndex` 1)
                          (`self.RemoveDialogueProgress` 2)
                          (`self.CloseConversation`))))))))
            (:`1`
              ;[1 1 1] Comment
              (`self.ClearDialogueProgress`)
              (`self.CloseConversation`))))))
    (:`1`
      ;[1 1 1] Comment
      (bind (_state_5 _optionindex_3) (`self.AddDialogue` "음치 건덕" "꽉 꽉 꽉꽉꽉 꽉(나에게 다시 말을 건거면 도와줄려는거지?)" (`|MakeArray` "그래!" "아니..." :!type "Text")))
      (switch `/Game/Blueprints/Dialogue/Enum_DialogueState` _state_5
        (:`NewEnumerator0`
          (switch `int` _optionindex_3
            (:`0`
              ;[1 1 1] Comment
              (bind _state_6 (`self.AddDialogue` "음치 건덕" "꽉꽉!(좋았어 가보는거야!)"))
              (switch `/Game/Blueprints/Dialogue/Enum_DialogueState` _state_6
                (:`NewEnumerator0`
                  (`self.SetDialogueTreeIndex` 2)
                  (`self.CloseConversation`)
                  (`GameplayStatics.OpenLevel` "MiniGame_Rhythm"))))
            (:`1`
              ;[1 1 1] Comment
              (bind _state_7 (`self.AddDialogue` "음치 건덕" "꽈악...(못된 인간놈...)" (`|MakeArray` "대화 끝내기" :!type "Text")))
              (switch `/Game/Blueprints/Dialogue/Enum_DialogueState` _state_7
                (:`NewEnumerator0`
                  (`self.RemoveDialogueProgress` 2)
                  (`self.CloseConversation`))))))))
    (:`2`
      ;[1 1 1] Comment
      (bind _state_8 (`self.AddDialogue` "음치 건덕" (select `int` (`KismetMathLibrary.RandomIntegerInRange` 0 1) :`0` "꽉 꽉!(안녕? 또 왔구나!)" :`1` "꽉꽉꽉?(내 노래를 들으러 와준거야?)" :!type "Text") (`|MakeArray` "대화 끝내기" :!type "Text")))
      (switch `/Game/Blueprints/Dialogue/Enum_DialogueState` _state_8
        (:`NewEnumerator0`
          (`self.RemoveDialogueProgress` 2)
          (`self.CloseConversation`))))))