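; Dialogue component for a waiting high school girl NPC who asks the player to check a rumor of objects moving at night in the engineering building.
; DialogueTreeIndex selects the branching intro, a re-offer after the rumor is dismissed, or random closing lines once accepted.
; Accepting sets the closing state, closes the conversation, calls ConnectToWebSocketAlive on KUGameInstance and shows MatchingWidget for the minigame.
; Other exits clear or roll back dialogue progress.
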(fn `Dialogue`
  (`parent.Dialogue`)
  (switch `int` (`self.DialogueTreeIndex`)
    (:`0`
      ;[1 1 1] Comment
      (bind (_state _optionindex) (`self.AddDialogue` "여자고등학생" "언니네 대학교 엄청 크다~ 나 궁금한거 있는데 물어봐도 돼?" (`|MakeArray` "응 그래." "아니." :!type "Text")))
      (switch `/Game/Blueprints/Dialogue/Enum_DialogueState` _state
        (:`NewEnumerator0`
          (switch `int` _optionindex
            (:`0`
              ;[1 1 1] Comment
              (bind (_state_2 _optionindex_2) (`self.AddDialogue` "여자고등학생" "우리 고등학교에서 소문으로는 공학관에서 밤에 사물들이 움직인다던데 알고 있어?" (`|MakeArray` "들은 적이 있다." "그런 터무니 없는 소리 하지마라." :!type "Text")))
              (switch `/Game/Blueprints/Dialogue/Enum_DialogueState` _state_2
                (:`NewEnumerator0`
                  (switch `int` _optionindex_2
                    (:`0`
                      ;[1 1 1] Comment
                      (bind _state_3 (`self.AddDialogue` "여자고등학생" "그러면 언니가 가서 확인해주고 와줘!" (`|MakeArray` "(미니게임 플레이)" :!type "Text")))
                      (switch `/Game/Blueprints/Dialogue/Enum_DialogueState` _state_3
                        (:`NewEnumerator0`
                          (`self.SetDialogueTreeIndex` 2)
                          (`self.CloseConversation`)
                          (bind _askugame_instance (cast `KUGameInstance` (`GameplayStatics.GetGameInstance`)))
                          (`KUGameInstance.ConnectToWebSocket_Alive` _askugame_instance "" 0)
                          (bind _returnvalue (`|CreateWidget` "/Game/BluePrint/Actors/UI/MatchingWidget.MatchingWidget_C"))
                          (`UserWidget.AddToViewport` _returnvalue 0))))
                    (:`1`
                      ;[1 1 1] Comment
                      (bind _state_4 (`self.AddDialogue` "여자고등학생" "재미 없어..." (`|MakeArray` "대화 끝내기" :!type "Text")))
                      (switch `/Game/Blueprints/Dialogue/Enum_DialogueState` _state_4
                        (:`NewEnumerator0`
                          (`self.SetDialogueTreeIndex` 1)
                          (`self.RemoveDialogueProgress` 2)
                          (`self.CloseConversation`))))))))
            (:`1`
              ;[1 1 1] Comment
              (`self.ClearDialogueProgress`)
              (`self.CloseConversation`))))))
    (:`1`
      ;[1 1 1] Comment
      (bind (_state_5 _optionindex_3) (`self.AddDialogue` "여자고등학생" "뭐야 다시 흥미가 생긴거야?" (`|MakeArray` "응." "아니..." :!type "Text")))
      (switch `/Game/Blueprints/Dialogue/Enum_DialogueState` _state_5
        (:`NewEnumerator0`
          (switch `int` _optionindex_3
            (:`0`
              ;[1 1 1] Comment
              (bind _state_6 (`self.AddDialogue` "여자고등학생" "갔다오고 말 좀 전해줘~"))
              (switch `/Game/Blueprints/Dialogue/Enum_DialogueState` _state_6
                (:`NewEnumerator0`
                  (`self.SetDialogueTreeIndex` 2)
                  (`self.CloseConversation`)
                  (bind _askugame_instance_2 (cast `KUGameInstance` (`GameplayStatics.GetGameInstance`)))
                  (`KUGameInstance.ConnectToWebSocket_Alive` _askugame_instance_2 "" 0)
                  (bind _returnvalue_2 (`|CreateWidget` "/Game/BluePrint/Actors/UI/MatchingWidget.MatchingWidget_C"))
                  (`UserWidget.AddToViewport` _returnvalue_2 0))))
            (:`1`
              ;[1 1 1] Comment
              (bind _state_7 (`self.AddDialogue` "여자고등학생" "난 여기 계쏙 있을게~" (`|MakeArray` "대화 끝내기" :!type "Text")))
              (switch `/Game/Blueprints/Dialogue/Enum_DialogueState` _state_7
                (:`NewEnumerator0`
                  (`self.RemoveDialogueProgress` 2)
                  (`self.CloseConversation`))))))))
    (:`2`
      ;[1 1 1] Comment
      (bind _state_8 (`self.AddDialogue` "여자고등학생" (select `int` (`KismetMathLibrary.RandomIntegerInRange` 0 1) :`0` "나 진짜 무섭다.." :`1` "그게 진짜였다니...." :!type "Text") (`|MakeArray` "대화 끝내기" :!type "Text")))
      (switch `/Game/Blueprints/Dialogue/Enum_DialogueState` _state_8
        (:`NewEnumerator0`
          (`self.RemoveDialogueProgress` 2)
          (`self.CloseConversation`))))))