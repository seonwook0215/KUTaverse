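; Dialogue component for the NPC 빛나, who asks the player to find something lost near 일감호 (Ilgam Lake).
; It overrides Dialogue, branching on DialogueTreeIndex into first request, repeat request or thanks, using chained AddDialogue calls.
; Accepting sets the thanks state before opening MiniGame_Jump, so it does not depend on the minigame's result.
; Refusing the search leads to the repeat request; thanks lines are picked randomly.
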(fn `Dialogue`
  (`parent.Dialogue`)
  (switch `int` (`self.DialogueTreeIndex`)
    (:`0`
      ;[1 1 1] Comment
      (bind (_state _optionindex) (`self.AddDialogue` "빛나" "안녕하세요! 혹시 저좀 도와주실 수 있을까요?" (`|MakeArray` "도와준다." "도와주지 않는다." :!type "Text")))
      (switch `/Game/Blueprints/Dialogue/Enum_DialogueState` _state
        (:`NewEnumerator0`
          (switch `int` _optionindex
            (:`0`
              ;[1 1 1] Comment
              (bind (_state_2 _optionindex_2) (`self.AddDialogue` "빛나" "아 고마워요. 제가 일감호 주변에서 뭐를 잃어버린 것 같아서요.... 찾아봐주실 수 있을까요?" (`|MakeArray` "찾으러 가본다." "그건 좀...." :!type "Text")))
              (switch `/Game/Blueprints/Dialogue/Enum_DialogueState` _state_2
                (:`NewEnumerator0`
                  (switch `int` _optionindex_2
                    (:`0`
                      ;[1 1 1] Comment
                      (bind _state_3 (`self.AddDialogue` "빛나" "고마워요!" (`|MakeArray` "(미니게임 플레이)" :!type "Text")))
                      (switch `/Game/Blueprints/Dialogue/Enum_DialogueState` _state_3
                        (:`NewEnumerator0`
                          (`self.SetDialogueTreeIndex` 2)
                          (`self.CloseConversation`)
                          (`GameplayStatics.OpenLevel` "MiniGame_Jump"))))
                    (:`1`
                      ;[1 1 1] Comment
                      (bind _state_4 (`self.AddDialogue` "빛나" "어쩔 수 없죠...." (`|MakeArray` "대화 끝내기" :!type "Text")))
                      (switch `/Game/Blueprints/Dialogue/Enum_DialogueState` _state_4
                        (:`NewEnumerator0`
                          (`self.SetDialogueTreeIndex` 1)
                          (`self.RemoveDialogueProgress` 2)
                          (`self.CloseConversation`))))))))
            (:`1`
              ;[1 1 1] Comment
              (`self.ClearDialogueProgress`)
              (`self.CloseConversation`))))))
    (:`1`
      ;[1 1 1] Comment
      (bind (_state_5 _optionindex_3) (`self.AddDialogue` "빛나" "도와주실 마음이 드셨나요?" (`|MakeArray` "그래!" "아니..." :!type "Text")))
      (switch `/Game/Blueprints/Dialogue/Enum_DialogueState` _state_5
        (:`NewEnumerator0`
          (switch `int` _optionindex_3
            (:`0`
              ;[1 1 1] Comment
              (bind _state_6 (`self.AddDialogue` "빛나" "고마워요! 찾으면 꼭 연락해주세요!"))
              (switch `/Game/Blueprints/Dialogue/Enum_DialogueState` _state_6
                (:`NewEnumerator0`
                  (`self.SetDialogueTreeIndex` 2)
                  (`self.CloseConversation`)
                  (`GameplayStatics.OpenLevel` "MiniGame_Jump"))))
            (:`1`
              ;[1 1 1] Comment
              (bind _state_7 (`self.AddDialogue` "빛나" "아쉽네요..." (`|MakeArray` "대화 끝내기" :!type "Text")))
              (switch `/Game/Blueprints/Dialogue/Enum_DialogueState` _state_7
                (:`NewEnumerator0`
                  (`self.RemoveDialogueProgress` 2)
                  (`self.CloseConversation`))))))))
    (:`2`
      ;[1 1 1] Comment
      (bind _state_8 (`self.AddDialogue` "빛나" (select `int` (`KismetMathLibrary.RandomIntegerInRange` 0 1) :`0` "반가워요! 제 은인!" :`1` "덕분에 물건을 잘 찾았어요~" :!type "Text") (`|MakeArray` "대화 끝내기" :!type "Text")))
      (switch `/Game/Blueprints/Dialogue/Enum_DialogueState` _state_8
        (:`NewEnumerator0`
          (`self.RemoveDialogueProgress` 2)
          (`self.CloseConversation`))))))