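; Level-3 piece for a merge game: hitting a "Level3" actor destroys both, spawns BP_KOO_Level04 at the hit point with Y zeroed, adds score and plays a sound.
; Tick snaps the actor transform to its Sphere component and times overlap with "EndLine".
; Lingering there past a short threshold, or entering a third time, sends game over through the GameInstance's WebSocketHandler, shows the lose UI and switches to UI-only input.
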(event `self.Sphere.OnComponentHit`
  (params (HitComponent :type "PrimitiveComponent Object Reference") (OtherActor :type "Actor Object Reference") (OtherComp :type "PrimitiveComponent Object Reference") (NormalImpulse :type "Vector Structure") (Hit :type "HitResult Structure (by ref)"))
  (bind (_bblockinghit _binitialoverlap _time _distance _location) (`GameplayStatics.BreakHitResult` Hit))
  (bind _returnvalue (`KismetMathLibrary.MakeVector` (.x _location) 0.0 (.z _location)))
  (`|ExecutionSequence`
    (:`then_0`
      (if (`KismetSystemLibrary.IsValid` OtherActor)
        (if (`self.ActorHasTag` OtherActor "Level3")
          (`self.K2_DestroyActor` OtherActor)
          (`self.K2_DestroyActor`)
          (`|SpawnActorFromClass` "/Game/BluePrint/Actors/Koo_Level/BP_KOO_Level04.BP_KOO_Level04_C" (`KismetMathLibrary.Conv_VectorToTransform` _returnvalue) "Undefined" "MultiplyWithRoot" null null)
          (bind _asmygame_mode (cast `/Game/BluePrint/Control/MYGameMode` (`GameplayStatics.GetGameMode`)))
          (`/Game/BluePrint/Control/MYGameMode.AddScroe` _asmygame_mode 60)
          (`GameplayStatics.PlaySoundAtLocation` "/Game/Sounds/Combine.Combine" _returnvalue (struct) 1.0 1.0 0.0 null null null null))))))

(event `self.ReceiveTick`
  (params (DeltaSeconds :type "Float (single-precision)"))
  (`|ExecutionSequence`
    (:`then_0`
      (`self.K2_SetActorTransform` (`KismetMathLibrary.MakeTransform` (`SceneComponent.K2_GetComponentLocation` (`self.Sphere`)) (`SceneComponent.K2_GetComponentRotation` (`self.Sphere`))))
      (if (`self.IsOverLap`)
        (set `self.OverlapTime` (- (`KismetSystemLibrary.GetGameTimeInSeconds`) (`self.OverlapTimeStart`)))))
    (:`then_1`
      (if (> (`self.OverlapTime`) 1.1)
        (bind _askugame_instance (cast `KUGameInstance` (`GameplayStatics.GetGameInstance`)))
        (`KooWebSocketHandler.SendGameOver` (`KUGameInstance.WebSocketHandler` _askugame_instance))
        (bind _foundwidgets (`WidgetBlueprintLibrary.GetAllWidgetsOfClass` "/Game/BluePrint/Actors/UI/NewWidgetBlueprint.NewWidgetBlueprint_C"))
        (for _array_element _foundwidgets
          (`Widget.SetVisibility` (`/Game/BluePrint/Actors/UI/NewWidgetBlueprint.GameEndLose` _array_element) "Visible")
          (`WidgetBlueprintLibrary.SetInputMode_UIOnlyEx` (`GameplayStatics.GetPlayerController` 0) null))))))

(event `self.Sphere.OnComponentBeginOverlap`
  (params (OverlappedComponent :type "PrimitiveComponent Object Reference") (OtherActor :type "Actor Object Reference") (OtherComp :type "PrimitiveComponent Object Reference") (OtherBodyIndex :type Integer) (bFromSweep :type Boolean) (SweepResult :type "HitResult Structure (by ref)"))
  (if (`self.ActorHasTag` OtherActor "EndLine")
    (`|ExecutionSequence`
      (:`then_0`
        (set `self.IsOverLap` true)
        (set `self.OverlapTimeStart` (`KismetSystemLibrary.GetGameTimeInSeconds`)))
      (:`then_1`
        (if (>= (`self.Count`) 2)
          (bind _askugame_instance (cast `KUGameInstance` (`GameplayStatics.GetGameInstance`)))
          (`KooWebSocketHandler.SendGameOver` (`KUGameInstance.WebSocketHandler` _askugame_instance))
          (bind _foundwidgets (`WidgetBlueprintLibrary.GetAllWidgetsOfClass` "/Game/BluePrint/Actors/UI/NewWidgetBlueprint.NewWidgetBlueprint_C"))
          (for _array_element _foundwidgets
            (`Widget.SetVisibility` (`/Game/BluePrint/Actors/UI/NewWidgetBlueprint.GameEndLose` _array_element) "Visible")
            (`WidgetBlueprintLibrary.SetInputMode_UIOnlyEx` (`GameplayStatics.GetPlayerController` 0) null))
          (else
            (set `self.Count` (+ (`self.Count`) 1))))))))

(event `self.Sphere.OnComponentEndOverlap`
  (params (OverlappedComponent :type "PrimitiveComponent Object Reference") (OtherActor :type "Actor Object Reference") (OtherComp :type "PrimitiveComponent Object Reference") (OtherBodyIndex :type Integer))
  (if (`self.ActorHasTag` OtherActor "EndLine")
    (set `self.IsOverLap` false)
    (set `self.OverlapTimeStart` 0.0)))

(fn `UserConstructionScript`)