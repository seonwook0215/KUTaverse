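; BP_EndLine is an end-line actor that shifts vertically in steps, apparently intended as a game-over boundary.
; MoveDownEndLine records the Box position and sets IsMoving; Tick then offsets local Z by MoveSpeed until MoveDistance is covered.
; While moving, Tick also updates EndLineLoca slightly below the actor.
; Overlap events are empty; the "Koo"-tag height check sending game over through KooWebSocketHandler is disconnected and never runs.
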(event `self.ReceiveBeginPlay`
  (set `self.StartLocation` (`SceneComponent.K2_GetComponentLocation` (`self.Box`))))

(event `self.Box.OnComponentBeginOverlap`
  (params (OverlappedComponent :type "PrimitiveComponent Object Reference") (OtherActor :type "Actor Object Reference") (OtherComp :type "PrimitiveComponent Object Reference") (OtherBodyIndex :type Integer) (bFromSweep :type Boolean) (SweepResult :type "HitResult Structure (by ref)")))

(event `self.Box.OnComponentEndOverlap`
  (params (OverlappedComponent :type "PrimitiveComponent Object Reference") (OtherActor :type "Actor Object Reference") (OtherComp :type "PrimitiveComponent Object Reference") (OtherBodyIndex :type Integer)))

(event `self.ReceiveTick`
  (params (DeltaSeconds :type "Float (single-precision)"))
  (bind (_returnvalue_x _returnvalue_y _returnvalue_z) (`KismetMathLibrary.BreakVector` (`self.K2_GetActorLocation`)))
  (bind (_startlocation_x _startlocation_y _startlocation_z) (`KismetMathLibrary.BreakVector` (`self.StartLocation`)))
  (if (`self.IsMoving`)
    (set `self.EndLineLoca` (- _returnvalue_z 30.0))
    (`self.K2_AddActorLocalOffset` (`KismetMathLibrary.MakeVector` 0.0 0.0 (* (`self.MoveSpeed`) DeltaSeconds)))
    (if (>= (`KismetMathLibrary.Abs` (- _startlocation_z _returnvalue_z)) (`self.MoveDistance`))
      (set `self.IsMoving` false))))

(fn `MoveDown_EndLine`
  (set `self.StartLocation` (`SceneComponent.K2_GetComponentLocation` (`self.Box`)))
  (set `self.IsMoving` true))

(fn `UserConstructionScript`)