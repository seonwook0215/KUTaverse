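; Player controller for a touch drop game: sets up Enhanced Input and the cursor, then spawns KOO actors where the player taps.
; A tap, throttled by a timer cooldown, traces under the cursor and spawns the current level's Blueprint at fixed height, with X clamped per level.
; Each drop adds level-based score via MYGameMode, plays a click, randomly picks the next level favoring lower ones, and decrements BlockCount, which SetBlockCount replenishes.
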(event `self.ReceiveBeginPlay`
  (`EnhancedInputSubsystemInterface.AddMappingContext` (pcsubsystem `EnhancedInputLocalPlayerSubsystem` (`GameplayStatics.GetPlayerController` 0)) "/Game/BluePrint/Control/IMC_Default.IMC_Default" 0 (struct))
  (set `self.bShowMouseCursor` true)
  (bind _asmygame_mode (cast `/Game/BluePrint/Control/MYGameMode` (`GameplayStatics.GetGameMode`)))
  (set `self.As MYGame Mode` _asmygame_mode))

(event `EnhancedInput|/Game/BluePrint/Control/IA_Touch`
  (params (ActionValue :type Boolean) (ElapsedSeconds :type "Float (double-precision)") (TriggeredSeconds :type "Float (double-precision)") (InputAction :type "InputAction Object Reference" :default "/Game/BluePrint/Control/IA_Touch.IA_Touch"))
  (bind _locationx (`self.LocationX`))
  (bind _returnvalue (`KismetMathLibrary.MakeVector` _locationx 0.0 585.0))
  (:`Started`
    (if (`self.canClick`)
      (`KismetSystemLibrary.K2_SetTimer` null "ResertClickCooldown" 0.5)
      (set `self.canClick` false)
      (set `self.LocationX` (.x (`.Location` (`GameplayStatics.BreakHitResult` (`self.GetHitResultUnderCursorByChannel` (`GameplayStatics.GetPlayerController` 0) "TraceTypeQuery1" true)))))
      (switch `int` (`self.SpawnLevel`)
        (:`1`
          (if (<= _locationx 260.0)
            (if (>= _locationx -260.0)
              (bind _output_get (set `self.SpawnLoc` _returnvalue))
              (set `self.SpawnTransform` (`KismetMathLibrary.Conv_VectorToTransform` _output_get))
              (else
                (bind _output_get_2 (set `self.SpawnLoc` (-260.0 0.0 585.0)))
                (set `self.SpawnTransform` (`KismetMathLibrary.Conv_VectorToTransform` _output_get_2))))
            (else
              (bind _output_get_3 (set `self.SpawnLoc` (260.0 0.0 585.0)))
              (set `self.SpawnTransform` (`KismetMathLibrary.Conv_VectorToTransform` _output_get_3))))
          (`|SpawnActorFromClass` "/Game/BluePrint/Actors/Koo_Level/BP_KOO_Level01.BP_KOO_Level01_C" (`self.SpawnTransform`) "Undefined" "MultiplyWithRoot" null null)
          (`/Game/BluePrint/Control/MYGameMode.AddScroe` (`self.As MYGame Mode`) 10)
          (`GameplayStatics.PlaySound2D` "/Game/Sounds/Click.Click" 1.0 1.0 0.0 null null))
        (:`2`
          (if (<= _locationx 240.0)
            (if (>= _locationx -240.0)
              (bind _output_get_4 (set `self.SpawnLoc` _returnvalue))
              (set `self.SpawnTransform` (`KismetMathLibrary.Conv_VectorToTransform` _output_get_4))
              (else
                (bind _output_get_5 (set `self.SpawnLoc` (-240.0 0.0 585.0)))
                (set `self.SpawnTransform` (`KismetMathLibrary.Conv_VectorToTransform` _output_get_5))))
            (else
              (bind _output_get_6 (set `self.SpawnLoc` (240.0 0.0 585.0)))
              (set `self.SpawnTransform` (`KismetMathLibrary.Conv_VectorToTransform` _output_get_6))))
          (`|SpawnActorFromClass` "/Game/BluePrint/Actors/Koo_Level/BP_KOO_Level02.BP_KOO_Level02_C" (`self.SpawnTransform`) "Undefined" "MultiplyWithRoot" null null)
          (`/Game/BluePrint/Control/MYGameMode.AddScroe` (`self.As MYGame Mode`) 20)
          (`GameplayStatics.PlaySound2D` "/Game/Sounds/Click.Click" 1.0 1.0 0.0 null null))
        (:`3`
          (if (<= _locationx 220.0)
            (if (>= _locationx -220.0)
              (bind _output_get_7 (set `self.SpawnLoc` _returnvalue))
              (set `self.SpawnTransform` (`KismetMathLibrary.Conv_VectorToTransform` _output_get_7))
              (else
                (bind _output_get_8 (set `self.SpawnLoc` (-220.0 0.0 585.0)))
                (set `self.SpawnTransform` (`KismetMathLibrary.Conv_VectorToTransform` _output_get_8))))
            (else
              (bind _output_get_9 (set `self.SpawnLoc` (220.0 0.0 585.0)))
              (set `self.SpawnTransform` (`KismetMathLibrary.Conv_VectorToTransform` _output_get_9))))
          (`|SpawnActorFromClass` "/Game/BluePrint/Actors/Koo_Level/BP_KOO_Level03.BP_KOO_Level03_C" (`self.SpawnTransform`) "Undefined" "MultiplyWithRoot" null null)
          (`/Game/BluePrint/Control/MYGameMode.AddScroe` (`self.As MYGame Mode`) 30)
          (`GameplayStatics.PlaySound2D` "/Game/Sounds/Click.Click" 1.0 1.0 0.0 null null)))
      (if (<= (`KismetMathLibrary.RandomFloatInRange` 0.0 1.0) 0.5)
        (set `self.SpawnLevel` 1)
        (elif (<= (`KismetMathLibrary.RandomFloatInRange` 0.0 1.0) 0.6)
          (set `self.SpawnLevel` 2)
          (else
            (set `self.SpawnLevel` 3))))
      (if (> (`self.BlockCount`) 0)
        (set `self.BlockCount` (- (`self.BlockCount`) 1))))))

(fn `ResertClickCooldown`
  (set `self.canClick` true))

(fn `SetBlockCount`
  (set `self.BlockCount` (+ (`self.BlockCount`) 3)))

(fn `UserConstructionScript`)